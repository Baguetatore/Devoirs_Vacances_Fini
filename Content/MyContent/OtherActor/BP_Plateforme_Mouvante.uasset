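; Moving platform actor that travels when the player character touches its Box trigger, locking player input during the ride.
; BeginPlay caches player 0's MyCharacter, and the Box overlap disables its input and plays a Timeline.
; The Timeline track sets the Cube's relative location without sweep, then re-enables input on finish.
; An InterpToMovement activation branch remains in the graph but never runs.
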(event OnComponentBeginOverlap(Box)
  (params (OverlappedComponent :type Primitive%20Component%20Object%20Reference) (OtherActor :type Actor%20Object%20Reference) (OtherComp :type Primitive%20Component%20Object%20Reference) (OtherBodyIndex :type Integer) (bFromSweep :type Boolean) (SweepResult :type Hit%20Result%20Structure%20%28by%20ref%29))
  (bind _mycharacter_ref (Variables|Default|GetMyCharacter_Ref))
  ;[0.15 0.15 0.15 0.5] Lorsque le joueur touche la plateforme elle se déplace et les commandes sont désactivées durant le déplacement
  (if (== _mycharacter_ref OtherActor)
    (Input|DisableInput _mycharacter_ref 0)
    (bind _newtrack_0 (Timeline|Timeline Play)
      (:Update
        (Transformation|SetRelativeLocation (Variables|Default|GetCube) _newtrack_0 false false))
      (:Finished
        (Input|EnableInput _mycharacter_ref 0)))))

(event EventBeginPlay
  (bind _asmy_character (Utilities|Casting|CastToMyCharacter (Game|GetPlayerCharacter 0)))
  (Variables|Default|SetMyCharacter_Ref _asmy_character))

(event Collision|EventActorBeginOverlap
  (params (OtherActor :type Actor%20Object%20Reference)))

(event EventTick
  (params (DeltaSeconds :type Float%20%28single-precision%29)))

(fn ConstructionScript)